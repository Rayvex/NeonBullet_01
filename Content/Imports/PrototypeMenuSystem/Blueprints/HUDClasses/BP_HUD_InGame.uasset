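; In-game HUD Blueprint that switches input mode, pause and mouse cursor as the game state changes.
; On BeginPlay it binds to the BP_GameInstance state-change event, then requests the InGameHUD state; Destroyed unbinds it.
; The In Game HUD state gives game-only input, unpaused with a hidden cursor.
; Pause Menu pauses, shows the cursor and uses game-and-UI input focused on the GameInstance's active widget.
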(event Custom|OnStateChanged
  (params (NewState :type EGameState%20Enum :default "NewEnumerator0"))
  (bind _returnvalue (Game|GetPlayerController 0))
  ;[0 1 1 0.5] Sets up HUD interaction systems upon receiving game state change event notifications
  (switch Utilities|FlowControl|Switch|SwitchonEGameState NewState
    (:NewEnumerator1
      (Input|SetInputModeGameOnly _returnvalue)
      (Game|SetGamePaused false)
      (Variables|/Script/Engine.PlayerController|SetbShowMouseCursor _returnvalue false))
    (:NewEnumerator6
      (bind _asbp_game_instance (Utilities|Casting|CastToBP_GameInstance (Game|GetGameInstance)))
      (Input|SetInputModeGameandUI _returnvalue (Default|GetActiveUIWidget _asbp_game_instance) "DoNotLock" true)
      (Game|SetGamePaused true)
      (Variables|/Script/Engine.PlayerController|SetbShowMouseCursor _returnvalue true))))

(event EventBeginPlay
  (bind _returnvalue (Game|GetGameInstance))
  ;[0 1 0 0.5] Initialization Protocols
  (Utilities|FlowControl|Sequence
    (:then_0
      (bind _asbp_game_instance (Utilities|Casting|CastToBP_GameInstance _returnvalue))
      (EventDispatchers|BindEventtoStateChanged _asbp_game_instance (delegate Custom|OnStateChanged)) ; Starts listening in on game state change event
    )
    (:then_1
      (bind _asbp_game_instance_2 (Utilities|Casting|CastToBP_GameInstance _returnvalue))
      (Default|SetGameState _asbp_game_instance_2 "NewEnumerator1") ; Requests the Game Instance to set the Main Menu game state
    )))

(event EventDestroyed
  (bind _asbp_game_instance (Utilities|Casting|CastToBP_GameInstance (Game|GetGameInstance)))
  (EventDispatchers|UnbindEventfromStateChanged _asbp_game_instance (delegate Custom|OnStateChanged)) ; Stops listening to Game State change events
)

(fn ConstructionScript)