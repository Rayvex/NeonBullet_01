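; Player controller from a prototype menu system that handles basic movement, mouse look and pause toggling.
; On BeginPlay it caches mouse sensitivity and Y-inversion from the game instance's gameplay settings, then applies them to yaw and pitch input.
; Movement axes drive player pawn 0 along the controller's forward and right vectors.
; The P key switches the game instance's state between in-game HUD and pause menu.
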(event EventBeginPlay
  (bind _asbp_game_instance (Utilities|Casting|CastToBP_GameInstance (Game|GetGameInstance)))
  (bind (_mousexsensitivity _mouseysensitivity _invertmousey_) (Default|GetGameplayParameters (Default|GetGameplaySettings _asbp_game_instance)))
  (Variables|MouseSettings|SetMouseXSensitivity _mousexsensitivity)
  (Variables|MouseSettings|SetMouseYSensitivity _mouseysensitivity)
  (Variables|MouseSettings|SetInvertMouseY? _invertmousey_))

(event Input|AxisEvents|InputAxisMoveForward
  (params (AxisValue :type Float%20%28single-precision%29))
  ;[0 1 1 0.5] Basic Input Controls
  (Pawn|Input|AddMovementInput (Game|Player|GetPlayerPawn 0) (Transformation|GetActorForwardVector) AxisValue false))

(event Input|AxisEvents|InputAxisMoveRight
  (params (AxisValue :type Float%20%28single-precision%29))
  ;[0 1 1 0.5] Basic Input Controls
  (Pawn|Input|AddMovementInput (Game|Player|GetPlayerPawn 0) (Transformation|GetActorRightVector) AxisValue false))

(event Input|AxisEvents|InputAxisMouseX
  (params (AxisValue :type Float%20%28single-precision%29))
  ;[0 1 1 0.5] Basic Input Controls
  (Class|PlayerController|AddYawInput (* AxisValue (Variables|MouseSettings|GetMouseXSensitivity))))

(event Input|AxisEvents|InputAxisMouseY
  (params (AxisValue :type Float%20%28single-precision%29))
  (bind _mouseysensitivity (Variables|MouseSettings|GetMouseYSensitivity))
  (bind _returnvalue (* AxisValue _mouseysensitivity))
  ;[0 1 1 0.5] Basic Input Controls
  (if (Variables|MouseSettings|GetInvertMouseY?)
    (bind _result (Math|Float|NegateFloat _returnvalue)
      (:%20%20
        (Class|PlayerController|AddPitchInput _result)))
    (else
      (Class|PlayerController|AddPitchInput _returnvalue))))

(event Input|KeyboardEvents|P
  (params (Key :type Key%20Structure))
  ;[0 1 1 0.5] Pause Game/Access In-Game Menu
  (:Pressed
    (bind _asbp_game_instance (Utilities|Casting|CastToBP_GameInstance (Game|GetGameInstance)))
    (switch Utilities|FlowControl|Switch|SwitchonEGameState (Variables|/Game/Imports/PrototypeMenuSystem/Blueprints/BP_GameInstance.BP_GameInstance_C|GetGameState _asbp_game_instance)
      (:NewEnumerator1
        (Default|SetGameState _asbp_game_instance "NewEnumerator6"))
      (:NewEnumerator6
        (Default|SetGameState _asbp_game_instance "NewEnumerator1")))))

(fn ConstructionScript)