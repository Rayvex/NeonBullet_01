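; EnemyPortal is a wave-spawner Blueprint that spawns EnemyDrone_BP enemies at its Portal component's location.
; It exposes separate first, second and third wave events, all with identical logic and no callers in this file.
; Each call counts the drones in the level with GetAllActorsOfClass and spawns one more only while fewer than a hundred exist.
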(event Custom|FirstWave
  ;[1 1 1] Spawn first wave
  (bind _outactors (Actor|GetAllActorsOfClass "/Game/Blueprint/EnemyDrone_BP.EnemyDrone_BP_C"))
  (if (< (Utilities|Array|Length _outactors) 100)
    (Game|SpawnActorfromClass "/Game/Blueprint/EnemyDrone_BP.EnemyDrone_BP_C" (Math|Transform|MakeTransform (Transformation|GetWorldLocation (Variables|Default|GetPortal)) "0, 0, 0" "1,1,1") "Undefined" 0 0)))

(event Custom|SecondWave
  ;[1 1 1] Spawn second wave
  (bind _outactors (Actor|GetAllActorsOfClass "/Game/Blueprint/EnemyDrone_BP.EnemyDrone_BP_C"))
  (if (< (Utilities|Array|Length _outactors) 100)
    (Game|SpawnActorfromClass "/Game/Blueprint/EnemyDrone_BP.EnemyDrone_BP_C" (Math|Transform|MakeTransform (Transformation|GetWorldLocation (Variables|Default|GetPortal)) "0, 0, 0" "1,1,1") "Undefined" 0 0)))

(event Custom|ThirdWave
  ;[1 1 1] Spawn third wave
  (bind _outactors (Actor|GetAllActorsOfClass "/Game/Blueprint/EnemyDrone_BP.EnemyDrone_BP_C"))
  (if (< (Utilities|Array|Length _outactors) 100)
    (Game|SpawnActorfromClass "/Game/Blueprint/EnemyDrone_BP.EnemyDrone_BP_C" (Math|Transform|MakeTransform (Transformation|GetWorldLocation (Variables|Default|GetPortal)) "0, 0, 0" "1,1,1") "Undefined" 0 0)))

(fn ConstructionScript)