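; Enemy drone character that damages the player on contact and can trigger game over.
; Each actor overlap with a PlayerCharacter_BP switches on PlayerHealth, subtracting one point unless it is already zero.
; At zero it flags and hides the player, plays a death sound, shows the GameOver_BP widget and loads Main_Menu after a short delay.
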(event EventBeginPlay)

(event Collision|EventActorBeginOverlap
  (params (OtherActor :type Actor%20Object%20Reference))
  (bind _asplayer_character_bp (Utilities|Casting|CastToPlayerCharacter_BP OtherActor))
  (switch int (Variables|/Game/Blueprint/PlayerCharacter_BP.PlayerCharacter_BP_C|GetPlayerHealth _asplayer_character_bp)
    (:Default
      (Variables|/Game/Blueprint/PlayerCharacter_BP.PlayerCharacter_BP_C|SetPlayerHealth _asplayer_character_bp (- (Variables|/Game/Blueprint/PlayerCharacter_BP.PlayerCharacter_BP_C|GetPlayerHealth _asplayer_character_bp) 1)))
    (:0
      (Variables|/Game/Blueprint/PlayerCharacter_BP.PlayerCharacter_BP_C|SetKillPlayer _asplayer_character_bp true)
      (Rendering|SetActorHiddenInGame _asplayer_character_bp true)
      (Audio|PlaySound2D "/Game/Imports/Sounds/die2.die2" 1.5 0.8 0.0 0 0)
      (bind _returnvalue (UserInterface|CreateWidget "/Game/Blueprint/UI/GameOver_BP.GameOver_BP_C" (Game|GetPlayerController 0)))
      (UserInterface|Viewport|AddtoViewport _returnvalue 0)
      (Utilities|FlowControl|Delay 2.0)
      (Game|OpenLevel(byName) "Main_Menu"))))

(event EventTick
  (params (DeltaSeconds :type Float%20%28single-precision%29)))

(fn ConstructionScript)