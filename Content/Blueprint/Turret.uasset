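; Turret actor that turns its Barrels component to face the first player's character while InRange is true.
; Tick stores the frame's delta time and calls TurretRotation, which eases the barrels toward a look-at rotation using RInterpTo at RotationSpeed.
; The target keeps pitch and yaw but zeroes roll.
; InRange is only read here, and the graph contains no firing logic.
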(event Custom|TurretRotation
  (bind _returnvalue (Game|GetPlayerCharacter 0))
  (bind _barrels (Variables|Default|GetBarrels))
  (bind _returnvalue_2 (Transformation|GetWorldLocation _barrels))
  (bind _returnvalue_3 (Transformation|GetActorLocation _returnvalue))
  (bind _returnvalue_4 (Math|Rotator|FindLookatRotation _returnvalue_2 _returnvalue_3))
  (bind (_roll _pitch _yaw) (Math|Rotator|BreakRotator _returnvalue_4))
  (if (Variables|Default|GetInRange)
    (Transformation|SetWorldRotation (Variables|Default|GetBarrels) (Math|Interpolation|RInterpTo (Transformation|GetWorldRotation (Variables|Default|GetBarrels)) (Math|Rotator|MakeRotator 0.0 _pitch _yaw) (Variables|Default|GetDeltaTime) (Variables|Default|GetRotationSpeed)) false false)))

(event EventBeginPlay)

(event Collision|EventActorBeginOverlap
  (params (OtherActor :type Actor%20Object%20Reference)))

(event EventTick
  (params (DeltaSeconds :type Float%20%28single-precision%29))
  (Variables|Default|SetDeltaTime DeltaSeconds)
  (CallFunction|TurretRotation))

(fn ConstructionScript)