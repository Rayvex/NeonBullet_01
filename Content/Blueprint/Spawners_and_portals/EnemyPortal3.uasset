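; Enemy portal actor that spawns a timed wave of EnemyDrone_BP drones, then destroys itself.
; BeginPlay starts a looping FirstWave timer, waits through the wave duration, then re-sets that timer as non-looping and immediately destroys the actor.
; Each FirstWave tick spawns a drone at the Portal component's world location, provided the count of all drones in the level is under a fixed cap.
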(event Custom|FirstWave
  ;[1 1 1] Spawn first wave
  (bind _outactors (Actor|GetAllActorsOfClass "/Game/Blueprint/EnemyDrone_BP.EnemyDrone_BP_C"))
  (if (< (Utilities|Array|Length _outactors) 100)
    (Game|SpawnActorfromClass "/Game/Blueprint/EnemyDrone_BP.EnemyDrone_BP_C" (Math|Transform|MakeTransform (Transformation|GetWorldLocation (Variables|Default|GetPortal)) "0, 0, 0" "1,1,1") "Undefined" 0 0)))

(event EventBeginPlay
  ;[1 1 1] Spawn rate
  (Utilities|Time|SetTimerbyFunctionName 0 "FirstWave" 3.0 true)
  ;[1 1 1] Duration of wave
  (Utilities|FlowControl|Delay 3e+01)
  (Utilities|Time|SetTimerbyFunctionName 0 "FirstWave" 3.0)
  (Actor|DestroyActor))

(fn ConstructionScript)