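; Player character Blueprint that aims at the mouse cursor, shoots, and tracks health against enemy bullets.
; Each tick, a WorldStatic trace under the cursor sets the actor's yaw.
; While Shoot is held, a Gate feeds a short Delay and FlipFlop that alternate bullet spawns between left and right muzzles.
; Enemy bullet overlaps decrement health and hide the bullet; a hit at zero health hides the player and pauses the game.
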(event EventBeginPlay
  ;[1 1 1] Player takes damage from EnemyBullet
  (Variables|Default|SetplayerHealth 3))

(event Collision|EventActorBeginOverlap
  (params (OtherActor :type Actor%20Object%20Reference))
  ;[1 1 1] Player takes damage from EnemyBullet
  (Utilities|Casting|CastToEnemyBullet_BP OtherActor)
  (switch int (Variables|Default|GetplayerHealth)
    (:Default
      (Variables|Default|SetplayerHealth (- (Variables|Default|GetplayerHealth) 1))
      (Rendering|SetActorHiddenInGame OtherActor true))
    (:0
      (Rendering|SetActorHiddenInGame true)
      (Game|SetGamePaused true))))

(event EventTick
  (params (DeltaSeconds :type Float%20%28single-precision%29))
  (bind _returnvalue (Game|GetPlayerController 0))
  (bind _spawn_left (Variables|Default|GetSpawn%20Left))
  (bind _spawn_right (Variables|Default|GetSpawn%20Right))
  (bind (_worldlocation _worlddirection) (Game|Player|ConvertMouseLocationToWorldSpace _returnvalue))
  (bind _returnvalue_2 (Transformation|GetWorldTransform _spawn_left))
  (bind _returnvalue_3 (Transformation|GetWorldTransform _spawn_right))
  (bind (_location _rotation) (Math|Transform|BreakTransform _returnvalue_3))
  (bind (_location_2 _rotation_2) (Math|Transform|BreakTransform _returnvalue_2))
  (Utilities|FlowControl|Sequence
    (:then_0
      ;[1 1 1] Mouse aim
      (bind _outhit (Collision|LineTraceForObjects _worldlocation (+ _worldlocation (* _worlddirection 5000)) (Utilities|Array|MakeArray "ObjectTypeQuery1") false 0 "None"))
      (Transformation|SetActorRotation (Math|Rotator|MakeRotator 0.0 0.0 (.yaw (Math|Rotator|FindLookatRotation (Transformation|GetActorLocation) (.Location (Collision|BreakHitResult _outhit)))))))
    (:then_1
      ;[1 1 1] Shooting
      (Utilities|FlowControl|Gate true
        (:Exit
          (Utilities|FlowControl|Delay 0.07)
          (Utilities|FlowControl|FlipFlop
            (:A
              (Game|SpawnActorfromClass "/Game/Blueprint/PlayerBullet_BP.PlayerBullet_BP_C" (Math|Transform|MakeTransform (Math|Vector|MakeVector (+ (.x _location_2) 3.0) (.y _location_2) (.z _location_2)) _rotation_2) "Undefined" 0 0))
            (:B
              (Game|SpawnActorfromClass "/Game/Blueprint/PlayerBullet_BP.PlayerBullet_BP_C" (Math|Transform|MakeTransform (Math|Vector|MakeVector (+ (.x _location) 3.0) (.y _location) (.z _location)) _rotation) "Undefined" 0 0))))))))

(event Input|ActionEvents|InputActionShoot
  (params (Key :type Key%20Structure))
  (bind _spawn_left (Variables|Default|GetSpawn%20Left))
  (bind _spawn_right (Variables|Default|GetSpawn%20Right))
  (bind _returnvalue (Transformation|GetWorldTransform _spawn_left))
  (bind _returnvalue_2 (Transformation|GetWorldTransform _spawn_right))
  (bind (_location _rotation) (Math|Transform|BreakTransform _returnvalue_2))
  (bind (_location_2 _rotation_2) (Math|Transform|BreakTransform _returnvalue))
  ;[1 1 1] Shooting
  (:Pressed
    (Utilities|FlowControl|Gate true) ; enters at Open
  )
  (:Released
    (Utilities|FlowControl|Gate true) ; enters at Close
  ))

(fn ConstructionScript)