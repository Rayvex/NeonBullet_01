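; Health pickup actor that restores one point of health to the player on touch.
; It spins slowly every tick, with rotation not scaled by delta time.
; When its HealthItem component overlaps PlayerCharacter_BP, it increments PlayerHealth only if below the cap of ten, then destroys itself, so it stays in the world when the player is at full health.
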(event OnComponentBeginOverlap(HealthItem)
  (params (OverlappedComponent :type Primitive%20Component%20Object%20Reference) (OtherActor :type Actor%20Object%20Reference) (OtherComp :type Primitive%20Component%20Object%20Reference) (OtherBodyIndex :type Integer) (bFromSweep :type Boolean) (SweepResult :type Hit%20Result%20Structure%20%28by%20ref%29))
  (bind _asplayer_character_bp (Utilities|Casting|CastToPlayerCharacter_BP OtherActor))
  (if (< (Math|Conversions|ToFloat(Integer) (Variables|/Game/Blueprint/PlayerCharacter_BP.PlayerCharacter_BP_C|GetplayerHealth _asplayer_character_bp)) 1e+01)
    (Variables|/Game/Blueprint/PlayerCharacter_BP.PlayerCharacter_BP_C|SetplayerHealth _asplayer_character_bp (Math|Float|Truncate (+ (Math|Conversions|ToFloat(Integer) (Variables|/Game/Blueprint/PlayerCharacter_BP.PlayerCharacter_BP_C|GetplayerHealth _asplayer_character_bp)) 1.0)))
    (Components|DestroyComponent (Variables|Default|GetHealthItem))
    (Actor|DestroyActor)))

(event EventBeginPlay)

(event Collision|EventActorBeginOverlap
  (params (OtherActor :type Actor%20Object%20Reference)))

(event EventTick
  (params (DeltaSeconds :type Float%20%28single-precision%29))
  (Transformation|AddActorLocalRotation "0,2.000000, 0" false false))

(fn ConstructionScript)